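; Player cube Blueprint that keeps a running score, shows it on screen and tracks the high score.
; BeginPlay creates the UI_Score widget and loads the high score from an existing SaveGameHighScore slot.
; Tick raises the score by a fixed step per frame, independent of delta time, and updates the widget.
; A matched or beaten high score is copied into a loaded or new save object, but never saved to the slot.
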(event EventBeginPlay
  (bind _shs_save (Variables|Default|GetSHS%20Save))
  (bind _returnvalue (UserInterface|CreateWidget "/Game/Blueprints/HUD/UI_Score.UI_Score_C"))
  (bind _output_get (Variables|Default|SetUI _returnvalue))
  (UserInterface|Viewport|AddtoViewport _output_get 0)
  (bind _returnvalue_2 (SaveGame|DoesSaveGameExist _shs_save))
  (if _returnvalue_2
    (bind _returnvalue_3 (SaveGame|LoadGamefromSlot _shs_save))
    (bind _output_get_2 (Variables|Default|SetSave%20High%20Score _returnvalue_3))
    (bind _assave_game_high_score (Utilities|Casting|CastToSaveGameHighScore _output_get_2))
    (Variables|Default|SetHigh%20Score (Variables|/Game/Blueprints/SaveGameHighScore.SaveGameHighScore_C|GetHigh%20Score _assave_game_high_score))))

(event EventTick
  (params (DeltaSeconds :type Float%20%28single-precision%29))
  (bind _output_get (Variables|Default|SetScore (+ (Variables|Default|GetScore) 0.02)))
  (Default|UpdateScore (Variables|Default|GetUI) (Math|Float|Truncate _output_get))
  (if (>= (Variables|Default|GetScore) (Variables|Default|GetHigh%20Score))
    (bind _output_get_2 (Variables|Default|SetHigh%20Score (Math|Float|Truncate (Variables|Default|GetScore))))
    (bind _returnvalue (SaveGame|DoesSaveGameExist (Variables|Default|GetSHS%20Save)))
    (if _returnvalue
      (bind _returnvalue_2 (SaveGame|LoadGamefromSlot (Variables|Default|GetSHS%20Save)))
      (bind _output_get_3 (Variables|Default|SetSave%20High%20Score _returnvalue_2))
      (bind _assave_game_high_score (Utilities|Casting|CastToSaveGameHighScore _output_get_3))
      (Variables|/Game/Blueprints/SaveGameHighScore.SaveGameHighScore_C|SetHigh%20Score _assave_game_high_score _output_get_2)
      (else
        (bind _returnvalue_3 (SaveGame|CreateSaveGameObject "/Game/Blueprints/SaveGameHighScore.SaveGameHighScore_C"))
        (bind _output_get_4 (Variables|Default|SetSave%20High%20Score _returnvalue_3))
        (bind _assave_game_high_score_2 (Utilities|Casting|CastToSaveGameHighScore _output_get_4))
        (Variables|/Game/Blueprints/SaveGameHighScore.SaveGameHighScore_C|SetHigh%20Score _assave_game_high_score_2 _output_get_2)))))

(fn ConstructionScript)